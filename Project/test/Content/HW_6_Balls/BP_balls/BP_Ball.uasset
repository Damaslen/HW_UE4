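; BP_Ball is a ball actor that travels in a straight line and bounces off whatever blocks it.
; Each Tick it moves by Direction times Speed times delta time, using a swept world offset rather than physics simulation.
; On a blocking hit it reflects Direction about the hit normal and reduces Speed by the hit's Time value modulo a constant.
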(event EventBeginPlay)

(event Collision|EventActorBeginOverlap
  (params (OtherActor :type Actor%20Object%20Reference)))

(event EventTick
  (params (DeltaSeconds :type Float%20%28single-precision%29))
  (bind _sweephitresult (Transformation|AddActorWorldOffset (* (* (Variables|Default|GetDirection) (Variables|Default|GetSpeed)) DeltaSeconds) true))
  (if (.bBlockingHit (Collision|BreakHitResult _sweephitresult))
    (Variables|Default|SetDirection (Math|Vector|GetReflectionVector (Variables|Default|GetDirection) (.Normal (Collision|BreakHitResult _sweephitresult))))
    (if (.bBlockingHit (Collision|BreakHitResult _sweephitresult))
      (Variables|Default|SetSpeed (- (Variables|Default|GetSpeed) (Math|Float|%(Float) (.Time (Collision|BreakHitResult _sweephitresult)) 1e+01))))))

(fn ConstructionScript)